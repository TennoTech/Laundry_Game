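; BP_FinishArea is the level's finish area, where the player cashes in and the level outcome is decided.
; On BeginPlay it caches references to BP_Gamemode and the first player's BP_Player.
; Its CashIn function clears the passed player's elements and calls LevelCompleted on the game mode, flagging success when Score meets a hardcoded threshold.
; The file has no overlap or trigger logic of its own.
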(event EventBeginPlay
  (Utilities|FlowControl|Sequence
    (:then_0
      (bind _asbp_gamemode (Utilities|Casting|CastToBP_Gamemode (Game|GetGameMode)))
      (Variables|Default|SetGameModeRef _asbp_gamemode))
    (:then_1
      (bind _asbp_player (Utilities|Casting|CastToBP_Player (Game|GetPlayerCharacter 0)))
      (Variables|Default|SetPlayerRef _asbp_player))))

(fn ConstructionScript)

(fn Cashin
  (params (PlayerRef :type BP%20Player%20Object%20Reference))
  (Default|ClearElements PlayerRef)
  (Default|LevelCompleted (Variables|Default|GetGameModeRef) (>= (Variables|/Game/Blueprints/BP_Player.BP_Player_C|GetScore (Variables|Default|GetPlayerRef)) 5) (Variables|Default|GetPlayerRef)))