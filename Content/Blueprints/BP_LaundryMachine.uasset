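; BP_LaundryMachine is a washing machine that takes laundry from BP_Player and returns it after a timed cycle.
; StartMachine runs if the player's array has items, calling RemoveElements with WashedLaundry and starting a five-second timer to StopMachine.
; StopMachine flags the cycle complete, then CycleComplete calls AddElements on the player and clears that flag.
; Getters expose both state flags, and Tick prints the WashedLaundry count for debugging.
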(event EventBeginPlay
  (bind _asbp_player (Utilities|Casting|CastToBP_Player (Game|GetPlayerCharacter 0)))
  (Variables|Default|SetPlayerRef _asbp_player))

(event EventTick
  (params (DeltaSeconds :type Float%20%28single-precision%29))
  (Development|PrintString (Utilities|String|Append "CycleCompleted " (Utilities|String|ToString(Integer) (Utilities|Array|Length (Variables|Default|GetWashedLaundry)))) true true "(R=0.000000,G=0.660000,B=1.000000,A=1.000000)" 0.0))

(fn ConstructionScript)

(fn StartMachine
  (bind _playerref (Variables|Default|GetPlayerRef))
  (if (not (Default|ArrayEmpty _playerref))
    (Variables|Default|SetbIsMachineRunning true)
    (Default|RemoveElements _playerref (Variables|Default|GetWashedLaundry))
    (Utilities|Time|SetTimerbyFunctionName 0 "StopMachine" 5.0)))

(fn StopMachine
  (Variables|Default|SetbIsMachineRunning false)
  (Variables|Default|SetbIsCycleCompleted true))

(fn CycleComplete
  (Default|AddElements (Variables|Default|GetPlayerRef) (Variables|Default|GetWashedLaundry))
  (Variables|Default|SetbIsCycleCompleted false))

(fn GetIsMachineRunning
  (return (Variables|Default|GetbIsMachineRunning)))

(fn GetIsCycleCompleted
  (return (Variables|Default|GetbIsCycleCompleted)))