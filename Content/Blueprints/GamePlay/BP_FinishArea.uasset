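; BP_FinishArea is the level's finish area, where the player cashes in carried elements for score.
; On BeginPlay it caches references to BP_Gamemode and BP_Player.
; CashIn skips when the player's Clean value is zero or less, otherwise clears their elements and compares the returned total to ScoreToPassLevel.
; Reaching the threshold completes the level through the game mode, while falling short posts a score progress notification.
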(event EventBeginPlay
  (Utilities|FlowControl|Sequence
    (:then_0
      (bind _asbp_gamemode (Utilities|Casting|CastToBP_Gamemode (Game|GetGameMode)))
      (Variables|Default|SetGameModeRef _asbp_gamemode))
    (:then_1
      (bind _asbp_player (Utilities|Casting|CastToBP_Player (Game|GetPlayerCharacter 0)))
      (Variables|Default|SetPlayerRef _asbp_player))))

(fn ConstructionScript)

(fn Cashin
  (params (PlayerRef :type BP%20Player%20Object%20Reference))
  (bind _scoretopasslevel (Variables|Default|GetScoreToPassLevel))
  (bind _clean (Default|GetArray PlayerRef))
  (if (not (<= _clean 0))
    (bind (_totalscore _amountadded) (Default|ClearElements PlayerRef))
    (if (>= _totalscore _scoretopasslevel)
      (Default|LevelCompleted (Variables|Default|GetGameModeRef))
      (else
        (Default|AddNotification (Variables|Default|GetGameModeRef) (Utilities|Text|FormatText "You Scored: {Amount} 
New Total: {Score} Out Of {PassLevelScore}" _amountadded _totalscore _scoretopasslevel))))))