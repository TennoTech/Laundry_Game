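; BP_PickUpBase is a base laundry pickup that carries a random coin value, set at BeginPlay, and a clean-state flag.
; Its construction script gives the mesh a dynamic material with a random color.
; On interact, it checks the player's carried count against MaxCarry, then either adds itself to the passed laundry array and hides without collision, or posts a basket-full notification through the player's game mode reference.
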(event EventBeginPlay
  (Variables|Default|SetCoins (Math|Random|RandomIntegerinRange 3 20)))

(fn ConstructionScript
  (bind _returnvalue (Rendering|Material|CreateDynamicMaterialInstance (Variables|Default|GetStaticMesh) 0 0 "None" :!class /Script/Engine.PrimitiveComponent))
  (Rendering|Material|SetVectorParameterValue _returnvalue "Color" (Utilities|Struct|MakeLinearColor (Math|Random|RandomFloatinRange 0.0 1.0) (Math|Random|RandomFloatinRange 0.0 1.0) (Math|Random|RandomFloatinRange 0.0 1.0) 0.0) :!class /Script/Engine.MaterialInstanceDynamic))

(fn GetCoins
  (return (Variables|Default|GetCoins)))

(fn SetIsClean
  (params (bIsClean :type Boolean))
  (Variables|Default|SetbIsClean bIsClean))

(fn GetIsClean
  (return (Variables|Default|GetbIsClean)))

(fn OnInteract
  (params (LaundryArray :type Array%20of%20BP%20Pick%20Up%20Base%20Object%20References) (PlayerRef :type BP%20Player%20Object%20Reference))
  (bind _totalcount (Default|GetArray PlayerRef))
  (if (<= _totalcount (Variables|/Game/Blueprints/BP_Player.BP_Player_C|GetMaxCarry PlayerRef))
    (Utilities|Array|Add LaundryArray self)
    (Rendering|SetActorHiddenInGame true)
    (Collision|SetActorEnableCollision false)
    (else
      (Default|AddNotification (Variables|/Game/Blueprints/BP_Player.BP_Player_C|GetGameModeRef PlayerRef) "Laundry Basket Full"))))