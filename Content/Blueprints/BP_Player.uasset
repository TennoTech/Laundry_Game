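; First-person player pawn for a laundry game that collects laundry, cleans it in machines and cashes it in for score.
; Interact line-traces from the camera; a basket must be picked up before pickups, laundry machines or the finish area respond.
; The Laundry array is the inventory, with helpers that hand dirty items out, take them back clean and convert clean ones to coins, firing count-change events.
; BeginPlay opens a tutorial widget in UI-only input mode.
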(event EventBeginPlay
  (bind _returnvalue (Game|GetPlayerController 0))
  (bind _returnvalue_2 (UserInterface|CreateWidget "/Game/Blueprints/Widgets/MainMenu/WBP_Tutorial.WBP_Tutorial_C"))
  (UserInterface|Viewport|AddtoViewport _returnvalue_2 0)
  (Variables|/Script/Engine.PlayerController|SetbShowMouseCursor _returnvalue true)
  (Input|SetInputModeUIOnly _returnvalue _returnvalue_2 "DoNotLock"))

(event EventTick
  (params (DeltaSeconds :type Float%20%28single-precision%29)))

(event Input|ActionEvents|InputActionInteract
  (params (Key :type Key%20Structure :default "None"))
  (bind _camera (Variables|Default|GetCamera))
  (bind _returnvalue (Transformation|GetWorldLocation _camera))
  (:Pressed
    (bind _outhit (Collision|LineTraceByChannel _returnvalue (+ _returnvalue (* (Math|Vector|GetForwardVector _camera) 1e+03)) "TraceTypeQuery1" false 0 "ForDuration"))
    (CallFunction|GetInteractingObject (.HitActor (Collision|BreakHitResult _outhit)))))

(event Input|AxisEvents|InputAxisMoveForward
  (params (AxisValue :type Float%20%28single-precision%29))
  (Pawn|Input|AddMovementInput (Math|Vector|GetForwardVector (Variables|Collision|GetCapsuleComponent)) AxisValue false))

(event Input|AxisEvents|InputAxisMoveRight
  (params (AxisValue :type Float%20%28single-precision%29))
  (Pawn|Input|AddMovementInput (Math|Vector|GetRightVector (Variables|Collision|GetCapsuleComponent)) AxisValue false))

(event Input|AxisEvents|InputAxisLookUp
  (params (AxisValue :type Float%20%28single-precision%29))
  (Pawn|Input|AddControllerPitchInput AxisValue))

(event Input|AxisEvents|InputAxisTurn
  (params (AxisValue :type Float%20%28single-precision%29))
  (Pawn|Input|AddControllerYawInput AxisValue))

(fn ConstructionScript)

(fn AddElements
  (params (Array :type Array%20of%20BP%20Pick%20Up%20Base%20Object%20References))
  (for _array_element Array
    (Default|SetIsClean _array_element true)
    (Utilities|Array|Add (Variables|Default|GetLaundry) _array_element))
  (Utilities|Array|Clear Array)
  (Default|CallOnLaundryCountChanged))

(fn RemoveElements
  (params (Array :type Array%20of%20BP%20Pick%20Up%20Base%20Object%20References) (MachineLimit :type Integer))
  (bind _laundry (Variables|Default|GetLaundry))
  (bind _arrayelement (Utilities|Array|ReverseforEachLoop _laundry)
    (:LoopBody
      (if (< (LocalVariables|GetLoopCount) MachineLimit)
        (bind _bisclean (Default|GetIsClean _arrayelement))
        (if (not _bisclean)
          (Utilities|Array|Add Array _arrayelement)
          (Utilities|Array|RemoveItem _laundry _arrayelement)
          (Math|Integer|IncrementInt (LocalVariables|GetLoopCount)))))
    (:Completed
      (Default|CallOnLaundryCountChanged))))

(fn ArrayEmpty
  (return (== (Utilities|Array|Length (Variables|Default|GetLaundry)) 0)))

(fn ClearElements
  (bind _arrayelement (Utilities|Array|ReverseforEachLoop (Variables|Default|GetLaundry))
    (:LoopBody
      (bind _bisclean (Default|GetIsClean _arrayelement))
      (if _bisclean
        (bind _coins (Default|GetCoins _arrayelement))
        (Variables|Default|SetScore (+ _coins (Variables|Default|GetScore)))
        (Utilities|Array|RemoveItem (Variables|Default|GetLaundry) _arrayelement)))
    (:Completed
      (Default|CallOnLaundryCountChanged))))

(fn GetArray
  (for _array_element (Variables|Default|GetLaundry)
    (bind _bisclean (Default|GetIsClean _array_element))
    (if _bisclean
      (bind _result (Math|Integer|IncrementInt (LocalVariables|GetCleanCount))
        (:%20%20
          (LocalVariables|SetCleanCount _result)))
      (else
        (bind _result_2 (Math|Integer|IncrementInt (LocalVariables|GetDirtyCount))
          (:%20%20
            (LocalVariables|SetDirtyCount _result_2))))))
  (return (+ (LocalVariables|GetCleanCount) (LocalVariables|GetDirtyCount)) (LocalVariables|GetCleanCount) (LocalVariables|GetDirtyCount)))

(fn GetInteractingObject
  (params (NewParam :type Object%20Object%20Reference))
  (bind _output_get (LocalVariables|SetCastingObject NewParam))
  (if (Variables|Default|GetbHasBasket)
    (bind _asbp_pick_up_base (Utilities|Casting|CastToBP_PickUpBase (LocalVariables|GetCastingObject))
      (:then
        (Default|OnInteract _asbp_pick_up_base (Variables|Default|GetLaundry))
        (Default|CallOnLaundryCountChanged))
      (:CastFailed
        (bind _asbp_laundry_machine (Utilities|Casting|CastToBP_LaundryMachine (LocalVariables|GetCastingObject))
          (:then
            (Default|OnInteract _asbp_laundry_machine))
          (:CastFailed
            (bind _asbp_finish_area (Utilities|Casting|CastToBP_FinishArea (LocalVariables|GetCastingObject)))
            (if (not (CallFunction|ArrayEmpty))
              (Default|Cashin _asbp_finish_area self))))))
    (else
      (bind _asbp_basket (Utilities|Casting|CastToBP_Basket _output_get))
      (Default|OnInteractBasket _asbp_basket)
      (Variables|Default|SetbHasBasket true)
      (Default|CallOnLaundryBasketPickedUp))))