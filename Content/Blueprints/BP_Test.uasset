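; BP_Test is a test actor that displays a 15-second countdown as world-space text facing the player.
; BeginPlay starts a one-shot timer whose bound event is empty, so nothing happens on expiry.
; Each Tick writes the timer's rounded remaining time to the TextRender and rotates it toward player character 0 with a look-at rotation.
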(event Custom|CustomEvent_0)

(event EventBeginPlay
  (bind _returnvalue (Utilities|Time|SetTimerbyEvent (delegate Custom|CustomEvent_0) 15.0)))

(event EventTick
  (params (DeltaSeconds :type Float%20%28single-precision%29))
  (bind _textrender (Variables|Default|GetTextRender))
  (Rendering|Components|TextRender|SetText (Variables|Default|GetTextRender) (Utilities|Text|ToText(Integer) (Math|Float|Round (Utilities|Time|GetTimerRemainingTimebyHandle (stale EventBeginPlay _returnvalue)))))
  (Transformation|SetWorldRotation _textrender (Math|Rotator|FindLookatRotation (Transformation|GetWorldLocation _textrender) (Transformation|GetActorLocation (Game|GetPlayerCharacter 0))) false false))

(fn ConstructionScript)